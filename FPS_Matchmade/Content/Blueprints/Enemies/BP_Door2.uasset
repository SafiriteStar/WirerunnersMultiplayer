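; BP_Door2 is a door actor that slides open or closed on interaction and can be broken by repeated hits.
; InteractDoor toggles the Opened flag and plays one of two timelines that nudge the actor along its right vector on each update, so travel depends on update count.
; BreakDoor counts hits and, from the third onward, prints a debug string and moves the door to the world origin instead of destroying it.
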(event Custom|InteractDoor
  (if (Variables|Default|Getopened)
    (Variables|Default|Setopened false)
    (Timeline|Timeline PlayFromStart
      (:Update
        (Transformation|SetActorLocation (- (Transformation|GetActorLocation) (* (Transformation|GetActorRightVector) 3.3)) false false)))
    (else
      (Variables|Default|Setopened true)
      (Timeline|Timeline_0 PlayFromStart
        (:Update
          (Transformation|SetActorLocation (+ (* (Transformation|GetActorRightVector) 3.3) (Transformation|GetActorLocation)) false false))))))

(event Custom|BreakDoor
  (bind _result (Math|Integer|IncrementInt (Variables|Default|Gethits))
    (:%20%20
      (if (>= _result 3)
        (Development|PrintString "Hello")
        (Transformation|SetActorLocation "0, 0, 0" false false)))))

(event EventBeginPlay)

(event Collision|EventActorBeginOverlap
  (params (OtherActor :type Actor%20Object%20Reference)))

(event EventTick
  (params (DeltaSeconds :type Float%20%28single-precision%29)))

(fn ConstructionScript)