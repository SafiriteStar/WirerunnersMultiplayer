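; Behavior tree decorator for enemy AI that passes when the controlled pawn is farther than AttackRange from the Target blackboard actor.
; PerformConditionCheck casts the owner to a Controller, measures the distance from its pawn to the target and returns the comparison.
; The execution-start event is empty, and disconnected nodes hold an unused InRange blackboard write and debug prints.
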(event EventReceiveExecutionStartAI
  (params (OwnerController :type AI%20Controller%20Object%20Reference) (ControlledPawn :type Pawn%20Object%20Reference)))

(fn PerformConditionCheck
  (params (OwnerActor :type Actor%20Object%20Reference))
  (bind _ascontroller (Utilities|Casting|CastToController OwnerActor))
  (return (> (Transformation|GetDistanceTo (Pawn|GetControlledPawn _ascontroller) (AI|BehaviorTree|GetBlackboardValueasActor (Variables|Default|GetTarget))) (Variables|Default|GetAttackRange))))