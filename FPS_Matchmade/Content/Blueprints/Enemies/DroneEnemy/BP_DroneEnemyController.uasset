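; AI controller for the drone enemy that runs the BT_DroneEnemy behavior tree and feeds it sight-based player detection.
; Perception updates write a sighted Player-tagged actor to the TargetActor blackboard key and set HasActor.
; Sighting any other actor clears only HasActor.
; Lost sight or a non-sight stimulus clears only TargetActor, leaving HasActor unchanged.
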(event OnTargetPerceptionUpdated(AIPerception)
  (params (Actor :type Actor%20Object%20Reference) (Stimulus :type AI%20Stimulus%20Structure))
  (bind _returnvalue (AI|GetBlackboard 0))
  (bind _returnvalue_2 (Utilities|Name|MakeLiteralName "TargetActor"))
  (bind _returnvalue_3 (Utilities|Name|MakeLiteralName "HasActor"))
  (bind _returnvalue_4 (Class|AIPerceptionSystem|GetSenseClassforStimulus Stimulus))
  (if (== _returnvalue_4 "/Script/AIModule.AISense_Sight")
    (if (.bSuccessfullySensed (Utilities|Struct|BreakAIStimulus Stimulus))
      (if (Actor|ActorHasTag Actor "Player")
        (AI|Components|Blackboard|SetValueasObject _returnvalue _returnvalue_2 Actor)
        (AI|Components|Blackboard|SetValueasBool _returnvalue _returnvalue_3 true)
        (else
          (AI|Components|Blackboard|SetValueasBool _returnvalue _returnvalue_3 false)))
      (else
        (AI|Components|Blackboard|SetValueasObject _returnvalue _returnvalue_2 0 :!label _label)))
    (else
      (goto _label))))

(event EventBeginPlay
  (AI|RunBehaviorTree "/Game/Blueprints/Enemies/DroneEnemy/BT_DroneEnemy.BT_DroneEnemy"))

(event EventTick
  (params (DeltaSeconds :type Float%20%28single-precision%29)))

(fn ConstructionScript)