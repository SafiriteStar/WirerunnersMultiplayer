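; BPC_Health is a health component that tracks CurrentHealth against MaxHealth, starting full on BeginPlay.
; RemoveHealth subtracts an amount, clamps the result between zero and MaxHealth, and returns whether health is depleted.
; AddHealth uses the same clamp but also subtracts its input, so a positive value lowers health despite the function's name.
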(event EventBeginPlay
  (Variables|Default|SetCurrentHealth (Variables|Default|GetMaxHealth)))

(event EventTick
  (params (DeltaSeconds :type Float%20%28single-precision%29)))

(fn RemoveHealth
  (params (Amount :type Float%20%28double-precision%29))
  (bind _output_get (Variables|Default|SetCurrentHealth (Math|Float|Clamp(Float) (- (Variables|Default|GetCurrentHealth) Amount) 0.0 (Variables|Default|GetMaxHealth))))
  (return (<= _output_get 0.0)))

(fn AddHealth
  (params (B :type Float%20%28double-precision%29))
  (Variables|Default|SetCurrentHealth (Math|Float|Clamp(Float) (- (Variables|Default|GetCurrentHealth) B) 0.0 (Variables|Default|GetMaxHealth))))